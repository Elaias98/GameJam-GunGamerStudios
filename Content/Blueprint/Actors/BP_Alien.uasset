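; BP_Alien is a side-scrolling player character that moves, jumps, shoots and takes damage.
; Enhanced Input from IMC_GameJam drives movement along world X, flipping control yaw to match acceleration, and triggers jumps on player character 0.
; Firing spawns a BP_Proyectil, gated by the Dispara flag and a short delay as cooldown.
; VidaAlien decrements health (Vida), prints it for debugging and destroys the actor at zero.
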(event `self.ReceiveBeginPlay`
  (`KismetSystemLibrary.PrintString` (`KismetStringLibrary.Conv_DoubleToString` (`self.Vida`)) true true (struct :`R` 0.012128 :`G` 1.0 :`A` 1.0) 50000000000.0)
  (bind _asplayer_controller (cast `PlayerController` (`self.GetController`)))
  (message `EnhancedInputSubsystemInterface.AddMappingContext` (pcsubsystem `EnhancedInputLocalPlayerSubsystem` _asplayer_controller) "/Game/IMC/IMC_GameJam.IMC_GameJam" 0 (struct)))

(event `EnhancedInput|/Game/Inputs/IA_Disparar`
  (params (ActionValue :type "Float (double-precision)") (ElapsedSeconds :type "Float (double-precision)") (TriggeredSeconds :type "Float (double-precision)") (InputAction :type "InputAction Object Reference" :default "/Game/Inputs/IA_Disparar.IA_Disparar"))
  (bind _returnvalue (`self.GetTransform`))
  (:`Triggered`
    (if (`self.Dispara?`)
      (`|SpawnActorFromClass` "/Game/Blueprint/Actors/BP_Proyectil.BP_Proyectil_C" (`KismetMathLibrary.MakeTransform` (`KismetMathLibrary.MakeVector` (.x (.location _returnvalue)) (.y (.location _returnvalue)) (+ (.z (.location _returnvalue)) -40.0)) (`KismetMathLibrary.MakeRotator` 0.0 0.0 (+ (.yaw (.rotation _returnvalue)) 180.0))) "Undefined" "MultiplyWithRoot" null (-30.0 0.0 0.0) null)
      (set `self.Dispara?` false)
      (`KismetSystemLibrary.Delay` 0.5)
      (set `self.Dispara?` true))))

(event `EnhancedInput|/Game/Inputs/IA_Movimiento`
  (params (ActionValue :type "Float (double-precision)") (ElapsedSeconds :type "Float (double-precision)") (TriggeredSeconds :type "Float (double-precision)") (InputAction :type "InputAction Object Reference" :default "/Game/Inputs/IA_Movimiento.IA_Movimiento"))
  (bind _returnvalue (`self.GetController`))
  (bind _returnvalue_x (`KismetMathLibrary.BreakVector` (`CharacterMovementComponent.GetCurrentAcceleration` (`self.CharacterMovement`))))
  (:`Triggered`
    (`self.AddMovementInput` (1.0 0.0 0.0) ActionValue)
    (`/Engine/EditorBlueprintResources/StandardMacros.CompareFloat` _returnvalue_x
      (:`>`
        (`Controller.SetControlRotation` _returnvalue (`KismetMathLibrary.MakeRotator` 0.0)))
      (:`<`
        (`Controller.SetControlRotation` _returnvalue (`KismetMathLibrary.MakeRotator` 0.0 0.0 180.0))))))

(event `/Game/Blueprint/Interfaces/BPI_VidaAlien.VidaAlien`
  (bind _output_get (set `self.Vida` (- (`self.Vida`) 1.0)))
  (`KismetSystemLibrary.PrintString` (`KismetStringLibrary.Conv_DoubleToString` _output_get) true true (struct :`G` 0.66 :`B` 1.0 :`A` 1.0) 5000000.0)
  (if (== (`self.Vida`) 0.0)
    (`self.K2_DestroyActor`)))

(event `EnhancedInput|/Game/Inputs/IA_Salto`
  (params (ActionValue :type Boolean) (ElapsedSeconds :type "Float (double-precision)") (TriggeredSeconds :type "Float (double-precision)") (InputAction :type "InputAction Object Reference" :default "/Game/Inputs/IA_Salto.IA_Salto"))
  (:`Triggered`
    (`self.Jump` (`GameplayStatics.GetPlayerCharacter` 0))))

(fn `UserConstructionScript`)